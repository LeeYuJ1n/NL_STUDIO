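; Player controller that moves the controlled pawn toward the mouse cursor while the mouse input action is held.
; BeginPlay shows the cursor, and the press and release events toggle the controller's EnableClickEvents property, which doubles as the held-state flag.
; While it is set, Tick traces the Visibility channel under the cursor and feeds movement input along the direction from the pawn to the hit location.
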(event EventBeginPlay
  (Variables|/Script/Engine.PlayerController|SetbShowMouseCursor (Game|GetPlayerController 0) true))

(event EventTick
  (params (DeltaSeconds :type Float%20%28single-precision%29))
  (bind _returnvalue (Pawn|GetControlledPawn))
  (if (Variables|Default|GetbEnableClickEvents)
    (Pawn|Input|AddMovementInput _returnvalue (Math|Vector|GetUnitDirection(Vector) (Transformation|GetActorLocation _returnvalue) (.Location (Collision|BreakHitResult (.HitResult (Game|Player|GetHitResultUnderCursorbyChannel "TraceTypeQuery1" true))))) 1.0 false)))

(event Input|ActionEvents|InputAction마우스
  (params (Key :type Key%20Structure :default "None"))
  (:Pressed
    (Variables|Default|SetbEnableClickEvents true))
  (:Released
    (Variables|Default|SetbEnableClickEvents false)))

(fn ConstructionScript)
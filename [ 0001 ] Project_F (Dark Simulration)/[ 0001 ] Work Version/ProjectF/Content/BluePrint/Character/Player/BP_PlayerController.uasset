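; Player controller that steers the controlled pawn toward the point under the mouse cursor.
; BeginPlay makes the cursor visible for player 0.
; While EnableClickEvents is true, Tick traces under the cursor on the Visibility channel and feeds the direction from pawn to hit location into AddMovementInput.
; Movement follows the cursor continuously, with no click check or pathfinding in the graph.
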(event EventBeginPlay
  ;[1 1 1] 게임이 시작되고 플레이어 캐릭터가 있으면 마우스 커서 보이게 하기
  (Variables|/Script/Engine.PlayerController|SetbShowMouseCursor (Game|GetPlayerController 0) true))

(event EventTick
  (params (DeltaSeconds :type Float%20%28single-precision%29))
  (bind _returnvalue (Pawn|GetControlledPawn))
  ;[1 1 1] 코멘트
  (if (Variables|Default|GetbEnableClickEvents) ; IF문\n만약 조건이 True이면 다음 코드 실행\nFalse이면 그대로 끝내기
    (Pawn|Input|AddMovementInput _returnvalue (Math|Vector|GetUnitDirection(Vector) (Transformation|GetActorLocation _returnvalue) (.Location (Collision|BreakHitResult (.HitResult (Game|Player|GetHitResultUnderCursorbyChannel "TraceTypeQuery1" true))))) 1.0 false) ; 캐릭터나 폰에 이동 입력을 추가하는 데 사용됩니다. \n이 노드는 방향 벡터와 스케일 값을 받아, 해당 방향으로 캐릭터를 이동시킵니다.
  ))

(fn ConstructionScript)
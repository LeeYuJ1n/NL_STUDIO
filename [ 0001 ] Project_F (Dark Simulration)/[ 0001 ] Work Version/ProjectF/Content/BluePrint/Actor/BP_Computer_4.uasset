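; BP_Computer_4 is an interactable computer actor that opens a UI when the player uses it up close.
; A Box overlap with BP_ThirdPersonCharacter enables the actor's input for player 0 and shows the BP_Interact_Info widget.
; Pressing Interact replaces that widget with BP_Computer_Interact.
; Leaving the box disables input, and each of these events calls RemoveAllWidgets, clearing the whole viewport UI.
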(event OnComponentBeginOverlap(Box)
  (params (OverlappedComponent :type Primitive%20Component%20Object%20Reference) (OtherActor :type Actor%20Object%20Reference) (OtherComp :type Primitive%20Component%20Object%20Reference) (OtherBodyIndex :type Integer) (bFromSweep :type Boolean) (SweepResult :type Hit%20Result%20Structure%20%28by%20ref%29))
  (Utilities|Casting|CastToBP_ThirdPersonCharacter OtherActor)
  (Input|EnableInput (Game|GetPlayerController 0))
  (Viewport|RemoveAllWidgets)
  (bind _returnvalue (UserInterface|CreateWidget "/Game/BluePrint/Widget/Interact/BP_Interact_Info.BP_Interact_Info_C"))
  (UserInterface|Viewport|AddtoViewport _returnvalue 0))

(event OnComponentEndOverlap(Box)
  (params (OverlappedComponent :type Primitive%20Component%20Object%20Reference) (OtherActor :type Actor%20Object%20Reference) (OtherComp :type Primitive%20Component%20Object%20Reference) (OtherBodyIndex :type Integer))
  (Utilities|Casting|CastToBP_ThirdPersonCharacter OtherActor)
  (Input|DisableInput (Game|GetPlayerController 0))
  (Viewport|RemoveAllWidgets))

(event EventBeginPlay)

(event Collision|EventActorBeginOverlap
  (params (OtherActor :type Actor%20Object%20Reference)))

(event EventTick
  (params (DeltaSeconds :type Float%20%28single-precision%29)))

(event Input|ActionEvents|InputActionInteract
  (params (Key :type Key%20Structure :default "None"))
  (:Pressed
    (Viewport|RemoveAllWidgets)
    (bind _returnvalue (UserInterface|CreateWidget "/Game/BluePrint/Widget/Interact/BP_Computer_Interact.BP_Computer_Interact_C"))
    (UserInterface|Viewport|AddtoViewport _returnvalue 0)))

(fn ConstructionScript)